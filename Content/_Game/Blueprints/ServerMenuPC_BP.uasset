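; Player controller for the server menu that relays lobby requests between the player and the server.
; On BeginPlay it caches the menu HUD and asks MyServerMenuGameModeBase to send the connected clients.
; Player list updates arrive through TriggerUpdatePlayerListFromServer, are stored, and reach the HUD's menu screen after a short delay.
; Launch requests pass through a handler event that calls ServerTravel with the given map path.
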(event `SendLaunchRequestToServer`
  (params (MapPath :type String))
  (`self.HandleLaunchRequestOnServer` MapPath))

(event `HandleLaunchRequestOnServer`
  (params (MapPath :type String))
  (`self.ServerTravel` MapPath))

(event `RequestConnectClientsFromServer`
  (`self.ServerTriggeredFromClientForConnectedPlayer`))

(event `ServerTriggeredFromClientForConnectedPlayer`
  (bind _asmy_server_menu_game_mode_base (cast `/Game/_Game/Blueprints/MyServerMenuGameModeBase` (`GameplayStatics.GetGameMode`)))
  (`/Game/_Game/Blueprints/MyServerMenuGameModeBase.SendConnectedClients` _asmy_server_menu_game_mode_base))

(event `self.ReceiveBeginPlay`
  (`KismetSystemLibrary.PrintString` "Hello")
  (bind _asserver_menu_hud (cast `/Game/_Game/Blueprints/ServerMenu_HUD` (`self.GetHUD`)))
  (set `self.As Server Menu HUD` _asserver_menu_hud)
  (`self.RequestConnectClientsFromServer`))

(event `UpdatePlayerList`
  (params (ConnectedPlayerInfo :type "Array of /Game/_Game/Blueprints/ServerMenuUI/F_PlayerInfo Structure"))
  (bind _output_get (set `self.Connected Player Info` ConnectedPlayerInfo))
  (`KismetSystemLibrary.PrintString` "TRIGGERED HERE")
  (`KismetSystemLibrary.Delay` 0.2)
  (`/Game/_Game/Blueprints/ServerMenuUI/ServerMenuInterface.UpdatePlayerList` (`/Game/_Game/Blueprints/ServerMenu_HUD.Server Menu Screen` (`self.As Server Menu HUD`)) _output_get))

(event `TriggerUpdatePlayerListFromServer`
  (params (ConnectedPlayers :type "Array of /Game/_Game/Blueprints/ServerMenuUI/F_PlayerInfo Structure"))
  (`self.UpdatePlayerList` ConnectedPlayers))

(fn `UserConstructionScript`)